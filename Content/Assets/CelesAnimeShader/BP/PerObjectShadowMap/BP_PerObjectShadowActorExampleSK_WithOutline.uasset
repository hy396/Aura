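; Example actor for per-object shadow mapping on a skeletal mesh with an outline, from the Celes anime shader assets.
; A shadow capture component is initialized with a light target, the skeletal mesh and a SceneCapture2D, both in construction and at BeginPlay.
; Construction also updates the shadow map for editor preview and makes a second skeletal mesh follow the main mesh's pose through leader pose.
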(event `self.ReceiveBeginPlay`
  (`/Game/Assets/CelesAnimeShader/BP/PerObjectShadowMap/AC_PerObjectShadowCaptureComp.InitShadowCapture` (`self.AC_PerObjectShadowCaptureComp`) (`self.LightTarget`) (`self.SkeletalMesh`) (`self.SceneCaptureComponent2D`)))

(fn `UserConstructionScript`
  (bind _ac_perobjectshadowcapturecomp (`self.AC_PerObjectShadowCaptureComp`))
  ;[1 1 1] In Editor Update
  (`/Game/Assets/CelesAnimeShader/BP/PerObjectShadowMap/AC_PerObjectShadowCaptureComp.InitShadowCapture` _ac_perobjectshadowcapturecomp (`self.LightTarget`) (`self.SkeletalMesh`) (`self.SceneCaptureComponent2D`))
  (`/Game/Assets/CelesAnimeShader/BP/PerObjectShadowMap/AC_PerObjectShadowCaptureComp.UpdateShadowmap` _ac_perobjectshadowcapturecomp)
  (`SkinnedMeshComponent.SetLeaderPoseComponent` (`self.SkeletalMesh1`) (`self.SkeletalMesh`) false false))