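; Example actor Blueprint that demonstrates per-object shadow mapping for a static mesh in the CelesAnimeShader asset.
; Its shadow capture component uses a SceneCaptureComponent2D to capture the Sphere mesh's shadow map.
; The construction script initializes the capture without a light target and updates the shadow map immediately.
; BeginPlay reinitializes it with the LightTarget, while Tick is unused.
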(event `self.ReceiveBeginPlay`
  (`/Game/Assets/CelesAnimeShader/BP/PerObjectShadowMap/AC_PerObjectShadowCaptureComp.InitShadowCapture` (`self.AC_PerObjectShadowCaptureComp`) (`self.LightTarget`) (`self.Sphere`) (`self.SceneCaptureComponent2D`)))

(fn `UserConstructionScript`
  (bind _ac_perobjectshadowcapturecomp (`self.AC_PerObjectShadowCaptureComp`))
  (`/Game/Assets/CelesAnimeShader/BP/PerObjectShadowMap/AC_PerObjectShadowCaptureComp.InitShadowCapture` _ac_perobjectshadowcapturecomp null (`self.Sphere`) (`self.SceneCaptureComponent2D`))
  (`/Game/Assets/CelesAnimeShader/BP/PerObjectShadowMap/AC_PerObjectShadowCaptureComp.UpdateShadowmap` _ac_perobjectshadowcapturecomp))