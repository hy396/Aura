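; Actor component that gives its owning Character a short forward blink dodge (shanbi), cached as a Character reference on BeginPlay.
; Shanbi line-traces forward on Visibility, then teleports the owner to the hit point or trace end, spawning Niagara effects including NS_Blink_Fire at the destination.
; It sets the mesh visible only to scene captures without restoring it, and zeroes vertical velocity afterward.
; The Shanbi call in the event graph is unwired.
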(event `self.ReceiveBeginPlay`
  (bind `_as角色` (cast `Character` (`self.GetOwner`)))
  (set `self.As角色` `_as角色`))

(fn `shanbi`
  (bind `_as角色` (`self.As角色`))
  (bind `_as角色_2` (`self.As角色`))
  (bind (_returnvalue_x _returnvalue_y _returnvalue_z) (`KismetMathLibrary.BreakVector` (`Actor.K2_GetActorLocation` (`self.As角色`))))
  (bind _returnvalue (`Actor.K2_GetActorLocation` `_as角色_2`))
  (bind _charactermovement (`Character.CharacterMovement` (`self.As角色`)))
  (bind (_returnvalue_x_2 _returnvalue_y_2) (`KismetMathLibrary.BreakVector` (`CharacterMovementComponent.GetLastUpdateVelocity` _charactermovement)))
  (`NiagaraFunctionLibrary.SpawnSystemAtLocation` null (`KismetMathLibrary.MakeVector` _returnvalue_x _returnvalue_y (- _returnvalue_z 30.0)))
  (`PrimitiveComponent.SetVisibleInSceneCaptureOnly` (`Character.Mesh` (`self.As角色`)) true)
  (bind (_outhit _returnvalue_2) (`KismetSystemLibrary.LineTraceSingle` _returnvalue (+ _returnvalue (* (`Actor.GetActorForwardVector` `_as角色_2`) 350)) "TraceTypeQuery1"))
  (if _returnvalue_2
    (bind (_bblockinghit _binitialoverlap _time _distance _location _impactpoint _normal _impactnormal _physmat _hitactor _hitcomponent _hitbonename _bonename _hititem _elementindex _faceindex _tracestart _traceend) (`GameplayStatics.BreakHitResult` _outhit))
    (`Actor.K2_SetActorLocation` `_as角色` (`KismetMathLibrary.MakeVector` (.x _location) (.y _location) (.z _location)) false false)
    (`NiagaraFunctionLibrary.SpawnSystemAtLocation` "/Game/Assets/BlinkAndDashVFX/VFX_Niagara/NS_Blink_Fire.NS_Blink_Fire" (`KismetMathLibrary.MakeVector` (.x _location) (.y _location) (- (.z _location) 30.0)))
    (else
      (`Actor.K2_SetActorLocation` `_as角色` (`KismetMathLibrary.MakeVector` (.x _traceend) (.y _traceend) (.z _traceend)) false false)
      (`NiagaraFunctionLibrary.SpawnSystemAtLocation` "/Game/Assets/BlinkAndDashVFX/VFX_Niagara/NS_Blink_Fire.NS_Blink_Fire" (`KismetMathLibrary.MakeVector` (.x _traceend) (.y _traceend) (- (.z _traceend) 30.0)))))
  (set `MovementComponent.Velocity` (`KismetMathLibrary.MakeVector` _returnvalue_x_2 _returnvalue_y_2) _charactermovement) ; 刷新一下速度
  (return))