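; BP_fuban is a test actor that moves vertically in an endless back-and-forth loop, apparently a floating platform.
; On BeginPlay it stores its Z, then 开始 (start) plays a timeline whose track value is added to that height.
; When finished, it saves the new Z and calls 结束 (end), whose second timeline subtracts its track value, then calls 开始 again.
; X and Y come from the current location throughout.
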(event `self.ReceiveBeginPlay`
  (set `self.Z` (.z (`self.K2_GetActorLocation`)))
  (`self.开始`))

(event `开始`
  (bind (_direction `_新建轨道_0`) (`Timeline|时间轴` :!via `PlayFromStart`)
    (:`Update`
      (bind _output_get (set `self.NewZ` (+ (`self.Z`) `_新建轨道_0`)))
      (`self.K2_SetActorLocation` (`KismetMathLibrary.MakeVector` (.x (`self.K2_GetActorLocation`)) (.y (`self.K2_GetActorLocation`)) _output_get)))
    (:`Finished`
      (set `self.Z` (`self.NewZ`))
      (`self.结束`))))

(event `结束`
  (bind (_direction `_新建轨道_0`) (`Timeline|时间轴_0` :!via `PlayFromStart`)
    (:`Update`
      (bind _output_get (set `self.NewZ` (- (`self.Z`) `_新建轨道_0`)))
      (`self.K2_SetActorLocation` (`KismetMathLibrary.MakeVector` (.x (`self.K2_GetActorLocation`)) (.y (`self.K2_GetActorLocation`)) _output_get)))
    (:`Finished`
      (set `self.Z` (`self.NewZ`))
      (`self.开始`))))

(fn `UserConstructionScript`)