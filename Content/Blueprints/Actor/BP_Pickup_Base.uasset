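; Base pickup actor that animates its spawn, hovers and spins, and destroys itself after DieTime.
; A timeline drives height and scale through UpdateLocationAndScale, with a one-shot impact sound at low elevation, then starts inherited rotation and sinusoidal movement.
; Tick applies CalculatedLocation and CalculatedRotation to the actor.
; Overlap logic is empty here; the consumed sound plays on any destruction, including timeout.
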(event `self.ReceiveBeginPlay`
  (`KismetSystemLibrary.K2_SetTimerDelegate` (delegate `消除Actor`) (`self.DieTime`))
  (`GameplayStatics.PlaySoundAtLocation` (`self.SpawnSound`) (`self.K2_GetActorLocation`) (struct) 1.0 1.0 0.0 null null null null) ; 播放生成音效
  (bind (_direction _elevation _scale) (`Timeline|时间轴`)
    (:`Update`
      (`self.UpdateLocationAndScale` _elevation _scale)
      (if (< _elevation 0.1)
        (`/Engine/EditorBlueprintResources/StandardMacros.DoOnce` false
          (:`Completed`
            (`GameplayStatics.PlaySoundAtLocation` (`self.GroundImpactSound`) (`self.K2_GetActorLocation`) (struct) 1.0 1.0 0.0 null null null null)))))
    (:`Finished`
      (`self.StartRotation`) ; 开始旋转
      (`self.StartSinusoidalMovement`) ; 开始移动
    )))

(event `消除Actor`
  (`self.K2_DestroyActor`))

(event `self.ReceiveTick`
  (params (DeltaSeconds :type "Float (single-precision)"))
  (`self.K2_SetActorLocation` (`self.CalculatedLocation`))
  (`self.K2_SetActorRotation` (`self.CalculatedRotation`)))

(event `self.ReceiveDestroyed`
  (`GameplayStatics.PlaySoundAtLocation` (`self.ConsumedSound`) (`self.K2_GetActorLocation`) (struct) 1.0 1.0 0.0 null null null null) ; 播放拾取音效
)

(fn `UpdateLocationAndScale`
  (params (Elevation :type "Float (double-precision)") (Scale :type "Float (single-precision)"))
  (bind (_calculatedlocation_x _calculatedlocation_y _calculatedlocation_z) (`KismetMathLibrary.BreakVector` (`self.CalculatedLocation`)))
  (`self.K2_SetActorLocation` (`KismetMathLibrary.MakeVector` _calculatedlocation_x _calculatedlocation_y (+ _calculatedlocation_z (* Elevation (`self.Spawn Apex`)))))
  (`self.SetActorScale3D` (`KismetMathLibrary.MakeVector` Scale Scale Scale)))

(fn `UserConstructionScript`)