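; Enemy summon ability that plays a shaman montage and spawns random minions at shuffled locations marked with Niagara effects.
; A montage gameplay event starts a delayed loop that spawns minions one by one, each given a controller and the avatar's level.
; Interface messages raise the avatar's minion count per spawn and lower it on destruction, which also resets the spawn index.
; The ability ends when the montage completes, is interrupted or is cancelled.
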(event `self.K2_ActivateAbility`
  (bind _returnvalue (`self.GetAvatarActorFromActorInfo`))
  (bind _output (`|GetArrayItem` (`self.Spawn Locations`) (`self.Spawn Location Index`)))
  (bind _returnvalue_2 (`self.GetSpawnLocations`))
  (bind _output_get (set `self.Spawn Locations` _returnvalue_2))
  (`KismetArrayLibrary.Array_Shuffle` _output_get)
  (for _array_element _output_get
    (`NiagaraFunctionLibrary.SpawnSystemAtLocation` "/Game/Assets/Effects/Combat/NS_Summon.NS_Summon" _array_element))
  (`AbilityTask_PlayMontageAndWait.CreatePlayMontageAndWaitProxy` "None" "/Game/Assets/Enemies/Shaman/Animations/AM_Shaman_Summon.AM_Shaman_Summon"
    (:`then`
      (`AbilityTask_WaitGameplayEvent.WaitGameplayEvent` (struct :`TagName` "Montage.Attack.1") null
        (:`EventReceived`
          (if (< (`self.Spawn Location Index`) (`KismetArrayLibrary.Array_Length` (`self.Spawn Locations`))) :!label _label
            (bind _returnvalue_3 (`|SpawnActorFromClass` (`self.GetRandomMinionClass`) (`KismetMathLibrary.MakeTransform` (+ _output (0.0 0.0 70.0)) (`KismetMathLibrary.FindLookAtRotation` (`Actor.K2_GetActorLocation` (`self.GetAvatarActorFromActorInfo`)) _output)) "AdjustIfPossibleButAlwaysSpawn" "MultiplyWithRoot" null null))
            (`Pawn.SpawnDefaultController` _returnvalue_3)
            (message `CombatInterface.IncrementMinionCount` _returnvalue 1)
            (bind _returnvalue_4 (message `CombatInterface.GetPlayerLevel` _returnvalue))
            (message `EnemyInterface.SetLevel` _returnvalue_3 _returnvalue_4)
            (add `Actor.OnDestroyed` _returnvalue_3 (delegate `OnDestroyed_Event`))
            (`/Engine/EditorBlueprintResources/StandardMacros.IncrementInt` (`self.Spawn Location Index`)
              (:`  `
                (`KismetSystemLibrary.Delay` 0.2)
                (goto _label)))))))
    (:`OnCompleted`
      (`self.K2_EndAbility` :!label _label_2))
    (:`OnInterrupted`
      (goto _label_2))
    (:`OnCancelled`
      (goto _label_2))))

(event `OnDestroyed_Event`
  (params (DestroyedActor :type "Actor Object Reference"))
  (message `CombatInterface.IncrementMinionCount` (`self.GetAvatarActorFromActorInfo`) -1)
  (set `self.Spawn Location Index` 0))