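; Enemy melee attack Gameplay Ability that turns the avatar toward its combat target and plays a random tagged attack montage.
; A gameplay event matching the montage's tag triggers a small sphere query at that montage's combat socket, damaging non-friendly live players found there.
; Any hit fires a MeleeImpact gameplay cue carrying the montage tag and location.
; The ability ends when the montage completes, is interrupted or is cancelled.
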(event `self.K2_ActivateAbility`
  (bind _returnvalue (`self.GetAvatarActorFromActorInfo`))
  (bind _returnvalue_2 (`self.GetAvatarActorFromActorInfo`))
  (set `self.HasHit Target` false)
  (bind _returnvalue_3 (message `EnemyInterface.GetCombatTarget` _returnvalue_2))
  (bind _ascombat_interface (cast `CombatInterface` _returnvalue_2)
    (:`then`
      (`CombatInterface.UpdateFacingTarget` _ascombat_interface (`Actor.K2_GetActorLocation` _returnvalue_3))
      (bind _returnvalue_4 (message `CombatInterface.GetAttackMontages` _returnvalue_2))
      (bind _output_get (set `self.TaggedMontage` (`self.GetRandomTaggedMontageFromArray` _returnvalue_4)))
      (bind (_montage _montagetag _sockettag) (break `TaggedMontage` _output_get))
      (`AbilityTask_PlayMontageAndWait.CreatePlayMontageAndWaitProxy` "None" _montage 1.0 "None" false
        (:`then`
          (`AbilityTask_WaitGameplayEvent.WaitGameplayEvent` _montagetag null
            (:`EventReceived`
              (bind _returnvalue_5 (message `CombatInterface.GetCombatSocketLocation` _returnvalue _sockettag))
              (bind _output_get_2 (set `self.Combat Location` _returnvalue_5))
              (bind _outoverlappingactors (`AuraAbilitySystemLibrary.GetLivePlayersWithinRadius` _returnvalue (`|MakeArray` _returnvalue) 45.0 _output_get_2))
              (for _array_element _outoverlappingactors
                (if (`AuraAbilitySystemLibrary.IsNotFriend` _array_element (`self.GetAvatarActorFromActorInfo`))
                  (`self.CauseDamage` _array_element)
                  (set `self.HasHit Target` true)))
              (if (`self.HasHit Target`)
                (bind _returnvalue_6 (message `EnemyInterface.GetCombatTarget` (`self.GetAvatarActorFromActorInfo`)))
                (`self.K2_ExecuteGameplayCueWithParams` (struct :`TagName` "GameplayCue.MeleeImpact") (`AbilitySystemBlueprintLibrary.MakeGameplayCueParameters` 0.0 0.0 (struct) (struct) (struct) (`BlueprintGameplayTagLibrary.MakeGameplayTagContainerFromTag` (`.MontageTag` (break `TaggedMontage` (`self.TaggedMontage`)))) (struct) (`self.Combat Location`) (0.0 0.0 0.0) null (`self.GetAvatarActorFromActorInfo`) _returnvalue_6))))))
        (:`OnCompleted`
          (`self.K2_EndAbility` :!label _label))
        (:`OnInterrupted`
          (goto _label))
        (:`OnCancelled`
          (goto _label))))
    (:`CastFailed`
      (`self.K2_EndAbility`))))