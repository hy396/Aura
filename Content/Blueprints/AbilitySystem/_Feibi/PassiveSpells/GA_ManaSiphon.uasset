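; GA_ManaSiphon is a passive gameplay ability that presents itself as mana regeneration (法力回复).
; It overrides GetDescription and GetNextLevelDescription to build rich-text tooltips showing the level, a once-per-second automatic mana restore, and no change at the next level.
; Activation and end events only call the parent, so the regeneration itself is not implemented in this graph.
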(event `self.K2_ActivateAbility`
  (`parent.K2_ActivateAbility`))

(event `self.K2_OnEndAbility`
  (params (bWasCancelled :type Boolean))
  (`parent.K2_OnEndAbility` bWasCancelled))

(fn `GetDescription`
  (params (Level :type Integer))
  (returns (ReturnValue :type String))
  (`parent.GetDescription` Level)
  (return (`KismetStringLibrary.Concat_StrStr` "<Title>法力回复</> \n<Small>等级：</> <Level>" (`KismetStringLibrary.Conv_IntToString` Level) "</> \n \n<Default>持续自动回复法力值，每</><Time>1s</><Default>一次。</>")))

(fn `GetNextLevelDescription`
  (params (Level :type Integer))
  (returns (ReturnValue :type String))
  (`parent.GetNextLevelDescription` Level)
  (return (`KismetStringLibrary.Concat_StrStr` "<Title>法力回复</> \n<Small>下一等级：</> <Level>" (`KismetStringLibrary.Conv_IntToString` Level) "</> \n \n<Default>无变化。 </> ")))