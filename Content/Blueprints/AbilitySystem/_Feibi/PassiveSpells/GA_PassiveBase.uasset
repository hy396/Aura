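; GA_PassiveBase is a base Gameplay Ability for passive spells that ties a gameplay effect to the ability's active lifetime.
; On activation it builds a spec from PassiveEffectClass at the ability's level and applies it to the owner's Ability System Component.
; When the ability ends it removes all stacks of that effect from the same component, matching by effect class rather than a stored handle.
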(event `self.K2_ActivateAbility`
  (`self.Apply GE`))

(event `self.K2_OnEndAbility`
  (params (bWasCancelled :type Boolean))
  (`self.Remove GE`))

(fn `Apply GE`
  (bind _returnvalue (`self.GetAbilitySystemComponentFromActorInfo`))
  (`AbilitySystemComponent.BP_ApplyGameplayEffectSpecToSelf` _returnvalue (`AbilitySystemComponent.MakeOutgoingSpec` :`self` _returnvalue :`GameplayEffectClass` (`self.PassiveEffectClass`) :`Level` (`KismetMathLibrary.Conv_IntToDouble` (`self.GetAbilityLevel`)))))

(fn `Remove GE`
  (`AbilitySystemComponent.RemoveActiveGameplayEffectBySourceEffect` (`self.GetAbilitySystemComponentFromActorInfo`) (`self.PassiveEffectClass`) null -1))