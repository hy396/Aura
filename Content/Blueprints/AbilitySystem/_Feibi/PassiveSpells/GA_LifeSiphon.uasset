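; Passive gameplay ability "Life Siphon", described to the player as continuous health regeneration once per second.
; Activation runs the parent logic and fires the LifeSiphon gameplay cue, while ending only defers to the parent.
; The regeneration itself is not implemented in this graph.
; Description overrides build Chinese rich-text strings showing the level, with the next-level text stating no change.
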(event `self.K2_ActivateAbility`
  (`parent.K2_ActivateAbility`)
  (`self.K2_ExecuteGameplayCue` (struct :`TagName` "GameplayCue.LifeSiphon")))

(event `self.K2_OnEndAbility`
  (params (bWasCancelled :type Boolean))
  (`parent.K2_OnEndAbility` bWasCancelled))

(fn `GetDescription`
  (params (Level :type Integer))
  (returns (ReturnValue :type String))
  (`parent.GetDescription` Level)
  (return (`KismetStringLibrary.Concat_StrStr` "<Title>生命回复</> \n<Small>等级：</>  <Level>" (`KismetStringLibrary.Conv_IntToString` Level) "</> \n \n<Default>持续自动回复生命值，每</><Time>1s</><Default>一次。</>")))

(fn `GetNextLevelDescription`
  (params (Level :type Integer))
  (returns (ReturnValue :type String))
  (`parent.GetNextLevelDescription` Level)
  (return (`KismetStringLibrary.Concat_StrStr` "<Title>生命回复</> \n<Small>下一等级：</>  <Level>" (`KismetStringLibrary.Conv_IntToString` Level) "</> \n \n<Default>无变化。 </> ")))