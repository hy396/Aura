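; Test fire bolt projectile for the ability system, built from a collision sphere, a fire effect and projectile movement.
; Shortly after BeginPlay it enables query-only collision on the sphere and spawns a Niagara shot effect just ahead of the actor.
; OnDestroy toggles the fire effect's visibility and deactivates projectile movement.
; The graph holds no hit or damage logic, as overlap and tick events are empty.
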(event `self.ReceiveBeginPlay`
  (bind _returnvalue (`self.GetTransform`))
  (`KismetSystemLibrary.Delay` 0.1)
  ;[1 1 1] 注释
  (bind _sphere (`self.Sphere`)
    (:`then`
      (`PrimitiveComponent.SetCollisionEnabled` _sphere "QueryOnly")
      (`NiagaraFunctionLibrary.SpawnSystemAtLocation` "/Game/Assets/_Niagara/Effect/NiagaraSystems/MagicTrailBullet/NS_Shot_01.NS_Shot_01" (`KismetMathLibrary.TransformLocation` _returnvalue (50.0 0.0 0.0)) (`KismetMathLibrary.TransformRotation` _returnvalue) (0.75 0.75 0.75)))
    (:`else`)))

(event `self.OnDestroy`
  (`SceneComponent.ToggleVisibility` (`self.FireEffect`) true)
  (`ActorComponent.Deactivate` (`self.ProjectileMovement`)))

(fn `UserConstructionScript`)