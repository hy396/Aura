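; BP_FireBolt1 is a fire bolt projectile for the ability system that plays a cast sound on spawn and enables query-only sphere collision after a brief delay.
; Each tick it compares its position with the previous frame, calling OnHit and destroying itself if it has barely moved.
; OnDestroy toggles the particle visibility, stops projectile movement and sets IsDead to end that check.
; Cast-effect spawning and delayed movement activation are left unconnected.
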(event `self.ReceiveBeginPlay`
  (`GameplayStatics.PlaySoundAtLocation` "/Game/Assets/_Niagara/VFX/Vefects/Anime_Stylized_VFX/Audio/MagicAttacks/SFX_MagicAttack_Fire_Cast_Cue.SFX_MagicAttack_Fire_Cast_Cue" (`self.K2_GetActorLocation`) (struct) 1.0 1.0 0.0 null null null null)
  (`KismetSystemLibrary.Delay` 0.05)
  (bind _sphere (`self.Sphere`)
    (:`then`
      (`PrimitiveComponent.SetCollisionEnabled` _sphere "QueryOnly"))
    (:`else`)))

(event `self.ReceiveTick`
  (params (DeltaSeconds :type "Float (single-precision)"))
  (if (not (`self.is Dead`))
    (`self.MakeGoKaboom ifNoMove`)))

(event `self.OnDestroy`
  (`SceneComponent.ToggleVisibility` (`self.ParticleSystem`) true)
  (`ActorComponent.Deactivate` (`self.ProjectileMovement`))
  (set `self.is Dead` true))

(fn `MakeGoKaboom ifNoMove`
  (set `self.Location Last Frame` (`self.Location This Frame`))
  (set `self.Location This Frame` (`self.K2_GetActorLocation`))
  (if (<= (`KismetMathLibrary.VSize` (- (`self.Location This Frame`) (`self.Location Last Frame`))) (`self.Min DistancePerFrame`))
    (`self.OnHit`)
    (`self.K2_DestroyActor`)))

(fn `UserConstructionScript`)