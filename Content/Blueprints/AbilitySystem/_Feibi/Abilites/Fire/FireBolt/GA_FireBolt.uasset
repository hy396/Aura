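; GA_FireBolt is a gameplay ability that casts fire bolt projectiles at the target under the mouse.
; It commits cost and cooldown on activation, turns the avatar toward the target data hit, then plays the attack montage.
; The montage's gameplay event triggers SpawnProjectiles from the weapon socket with an overridden upward pitch, passing the hit actor as homing target only if non-friendly.
; The ability ends when the montage finishes or is interrupted.
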(event `self.K2_ActivateAbility`
  (bind _returnvalue (`BlueprintGameplayTagLibrary.MakeLiteralGameplayTag` (struct :`TagName` "CombatSocket.Weapon")))
  (bind _homing_target (`self.Homing Target`))
  (bind _location (`self.Location`))
  (`self.K2_CommitAbility`) ; 启动Cost和Cooldown,我喜欢技能释放后出来在扣篮和cd
  (bind (_asynctaskproxy _datahandle) (`TargetDataUnderMouse.CreateTargetDataUnderMouse`)
    (:`ValidData`
      (bind (_bblockinghit _binitialoverlap _time _distance _location_2 _impactpoint _normal _impactnormal _physmat _hitactor) (`GameplayStatics.BreakHitResult` (`AbilitySystemBlueprintLibrary.GetHitResultFromTargetData` _datahandle)))
      (set `self.Location` _location_2)
      (set `self.Homing Target` _hitactor)
      (message `CombatInterface.UpdateFacingTarget` (`self.GetAvatarActorFromActorInfo`) (`self.Location`))
      (`AbilityTask_PlayMontageAndWait.CreatePlayMontageAndWaitProxy` "None" "/Game/Assets/Characters/Feibi/Anim/AM_AttackMontage.AM_AttackMontage" 1.0 "None" false
        (:`then`
          (`AbilityTask_WaitGameplayEvent.WaitGameplayEvent` (struct :`TagName` "Event.Montage.FireBolt") null true
            (:`EventReceived`
              (if (`AuraAbilitySystemLibrary.IsNotFriend` (`self.GetAvatarActorFromActorInfo`) _homing_target)
                (`self.SpawnProjectiles` _location _returnvalue true 45.0 _homing_target)
                (else
                  (`self.SpawnProjectiles` _location _returnvalue true 45.0 null))))))
        (:`OnCompleted`
          (`self.K2_EndAbility` :!label _label))
        (:`OnBlendOut`
          (goto _label))
        (:`OnInterrupted`
          (goto _label))
        (:`OnCancelled`
          (goto _label))))))