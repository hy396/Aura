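; BP_FireBlast is an ability-system fireball actor that flies out, returns to its caster and explodes nearby.
; On authority, one timeline lerps it forward to an apex, then a second homes back to the caster's current position.
; Within the explode distance, Boom calls OnHit, applies radial GAS damage to live players in radius except the owner, then destroys itself.
; Knockback and death impulse point away from the blast with a fixed upward pitch.
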(event `self.StartOutgoingTimeline`
  (`/Engine/EditorBlueprintResources/ActorMacros.Switch Has Authority`
    (:`Authority`
      ;[1 0.6274 0.07485] 存储起点和终点的位置
      (set `self.Initial Location` (`self.K2_GetActorLocation`)) ; 设置初始位置
      (set `self.Apex Location` (+ (`self.Initial Location`) (* (`self.GetActorForwardVector`) (`self.TravelDistance`))))
      (bind (_direction _outgoingtrack) (`Timeline|OutgoingTimeline`) ; 火球向外扩散
        (:`Update`
          (`self.K2_SetActorLocation` (`KismetMathLibrary.VLerp` (`self.Initial Location`) (`self.Apex Location`) _outgoingtrack)))
        (:`Finished`
          (bind (_direction_2 _returningtrack) (`Timeline|ReturningTimeline`) ; 火球返回角色
            (:`Update`
              (set `self.OwnerLocation` (`self.K2_GetActorLocation` (`self.ReturnToActor`))) ; 获取技能释放者的位置
              (`self.K2_SetActorLocation` (`KismetMathLibrary.VLerp` (`self.Apex Location`) (`self.OwnerLocation`) _returningtrack))
              (if (<= (`KismetMathLibrary.Vector_Distance` (`self.K2_GetActorLocation`) (`self.OwnerLocation`)) (`self.ExplodeDistance`))
                (`self.Boom`)))))))))

(fn `Apply GE To Actors`
  (params (`Attack Actors` :type "Array of Actor Object Reference"))
  (locals (`Overlap Actors` :type "Array of Actor Object Reference") (`Overlap Actor` :type "Actor Object Reference") (`Target ASC` :type "AbilitySystemComponent Object Reference") (`Atack Direction` :type "Vector Structure"))
  (bind _output_get (set `local.Overlap Actors` `Attack Actors`))
  (for _array_element _output_get
    (bind _output_get_2 (set `local.Overlap Actor` _array_element))
    (bind _output_get_3 (set `local.Target ASC` (`AbilitySystemBlueprintLibrary.GetAbilitySystemComponent` _output_get_2)))
    (if (`KismetSystemLibrary.IsValid` _output_get_3)
      (bind _output_get_4 (set `local.Atack Direction` (- (`self.K2_GetActorLocation` (`local.Overlap Actor`)) (`self.K2_GetActorLocation`)))) ; 获取击退朝向
      (bind (_returnvalue_roll _returnvalue_pitch _returnvalue_yaw) (`KismetMathLibrary.BreakRotator` (`KismetMathLibrary.MakeRotFromX` _output_get_4)))
      (set `local.Atack Direction` (`KismetMathLibrary.GetForwardVector` (`KismetMathLibrary.MakeRotator` _returnvalue_roll 45.0 _returnvalue_yaw))) ; 修改朝向
      (`AuraAbilitySystemLibrary.SetTargetEffectParamsASC` (`self.ExplosionDamageParams`) (`local.Target ASC`))
      (`AuraAbilitySystemLibrary.SetKnockbackDirection` (`self.ExplosionDamageParams`) (`local.Atack Direction`) (`self.KnockbackMagnitude`))
      (`AuraAbilitySystemLibrary.SetDeathImpulseDirection` (`self.ExplosionDamageParams`) (`local.Atack Direction`) (`self.DeathImpulseMagnitude`))
      (`AuraAbilitySystemLibrary.ApplyDamageEffect` (`self.ExplosionDamageParams`)))))

(fn `Boom`
  (bind _array (`|MakeArray` (`self.GetOwner`)))
  (`self.OnHit`)
  (`AuraAbilitySystemLibrary.SetIsRadialDamageEffectParam` (`self.ExplosionDamageParams`) true (`self.Radia Damage Inner Radius`) (`self.Radia Damage Outer Radius`) (`self.K2_GetActorLocation`))
  (`KismetArrayLibrary.Array_Add` _array self)
  (bind _outoverlappingactors (`AuraAbilitySystemLibrary.GetLivePlayersWithinRadius` (`self.GetOwner`) _array (`self.Radia Damage Outer Radius`) (`self.K2_GetActorLocation`)))
  (`self.Apply GE To Actors` _outoverlappingactors)
  (`self.K2_DestroyActor`))

(fn `UserConstructionScript`)