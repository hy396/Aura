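; BP_FireBolt is a fire projectile for the Barrage ability that launches after a short cast delay.
; On BeginPlay it spawns a Niagara cast effect just in front of itself and plays a fire cast sound.
; After the delay, nested validity checks gate enabling query-only sphere collision, activating projectile movement and toggling the bolt's Niagara visibility.
; This graph contains no hit or damage logic.
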(event `self.ReceiveBeginPlay`
  (bind _returnvalue (`self.GetTransform`))
  (bind _niagara (`self.Niagara`))
  (bind _projectilemovement (`self.ProjectileMovement`))
  ;[1 1 1] 注释
  (`NiagaraFunctionLibrary.SpawnSystemAtLocation` "/Game/Assets/_Niagara/VFX/Vefects/Anime_Stylized_VFX/Skills/MagicAttacks/Fire/NS_FireMagic_Cast.NS_FireMagic_Cast" (`KismetMathLibrary.TransformLocation` _returnvalue (50.0 0.0 0.0)) (`KismetMathLibrary.TransformRotation` _returnvalue))
  (`GameplayStatics.PlaySoundAtLocation` "/Game/Assets/_Niagara/VFX/Vefects/Anime_Stylized_VFX/Audio/MagicAttacks/SFX_MagicAttack_Fire_Cast_Cue.SFX_MagicAttack_Fire_Cast_Cue" (`self.K2_GetActorLocation`) (struct) 1.0 1.0 0.0 null null null null)
  (`KismetSystemLibrary.Delay` 0.9)
  (bind _sphere (`self.Sphere`)
    (:`then`
      (`PrimitiveComponent.SetCollisionEnabled` _sphere "QueryOnly")
      (`/Engine/EditorBlueprintResources/StandardMacros.IsValid` _projectilemovement
        (:`Is Valid`
          (`ActorComponent.Activate` _projectilemovement true) ; 激活运动
          (`/Engine/EditorBlueprintResources/StandardMacros.IsValid` _niagara
            (:`Is Valid`
              (`SceneComponent.ToggleVisibility` _niagara true))))))
    (:`else`)))

(fn `UserConstructionScript`)