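; GA_Barrage is a gameplay ability that fires a staggered volley of projectiles around the point under the mouse.
; It commits up front, turns the avatar toward the target, plays an attack montage and waits for the Barrage event.
; The event triggers a delayed loop spawning one projectile per spawn location with random XY target scatter.
; IsDaduan ends the ability if the montage finishes before that event; a homing spawn variant is disconnected.
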(event `self.K2_ActivateAbility`
  (bind _returnvalue (`KismetMathLibrary.RandomFloatInRange` -200.0 200.0))
  (`self.K2_CommitAbility`) ; 启动Cost和Cooldown,我喜欢技能释放后出来在扣篮和cd
  (bind (_asynctaskproxy _datahandle) (`TargetDataUnderMouse.CreateTargetDataUnderMouse`)
    (:`ValidData`
      (bind (_bblockinghit _binitialoverlap _time _distance _location _impactpoint _normal _impactnormal _physmat _hitactor) (`GameplayStatics.BreakHitResult` (`AbilitySystemBlueprintLibrary.GetHitResultFromTargetData` _datahandle)))
      (set `self.Location` _location)
      (set `self.Hit Actor` _hitactor)
      (bind _ascombat_interface (cast `CombatInterface` (`self.GetAvatarActorFromActorInfo`)))
      (`CombatInterface.UpdateFacingTarget` _ascombat_interface (`self.Location`))
      (`AbilityTask_PlayMontageAndWait.CreatePlayMontageAndWaitProxy` "None" "/Game/Assets/Characters/Feibi/Anim/AM_Attack02.AM_Attack02" 1.0 "None" false
        (:`then`
          (`AbilityTask_WaitGameplayEvent.WaitGameplayEvent` (struct :`TagName` "Event.Montage.Barrage") null true
            (:`EventReceived`
              (set `self.Is Daduan` false)
              (bind _returnvalue_2 (`self.GetSpawnLocations`))
              (set `self.Spawn Locations` _returnvalue_2)
              (if (< (`self.Spawn Location Index`) (`KismetArrayLibrary.Array_Length` (`self.Spawn Locations`))) :!label _label
                (`self.SpawnProjectile` (`|GetArrayItem` (`self.Spawn Locations`) (`self.Spawn Location Index`)) (`KismetMathLibrary.MakeVector` (+ (.x (`self.Location`)) _returnvalue) (+ (.y (`self.Location`)) _returnvalue) (.z (`self.Location`))))
                (`/Engine/EditorBlueprintResources/StandardMacros.IncrementInt` (`self.Spawn Location Index`)
                  (:`  `
                    (`KismetSystemLibrary.Delay` 0.1)
                    (goto _label)))
                (else
                  (`self.K2_EndAbility`))))))
        (:`OnCompleted`
          (if (`self.Is Daduan`) :!label _label_2
            (`self.K2_EndAbility`)))
        (:`OnBlendOut`
          (goto _label_2))
        (:`OnInterrupted`
          (goto _label_2))
        (:`OnCancelled`
          (goto _label_2))))))