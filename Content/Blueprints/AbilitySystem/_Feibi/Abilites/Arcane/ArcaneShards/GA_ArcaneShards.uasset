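; Arcane Shards gameplay ability: a targeted area attack that raises a series of damaging shards around a point picked with a magic circle.
; A second input press stores the cursor hit, spawns a BP_PointCollection for randomly rotated ground points, and plays a montage.
; The montage event commits cost and starts a looping timer, spawning one cue and radial damage with knockback per point.
; Shard count scales with ability level, capped; cooldown commits after the last shard.
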(event `self.K2_ActivateAbility`
  (bind _returnvalue (`self.K2_CheckAbilityCost`))
  (if _returnvalue
    (`|ExecutionSequence`
      (:`then_0`
        ;[0.05203 0.8096 1] 显示魔法阵，并隐藏鼠标
        (message `PlayerInterface.ShowMagicCircle` (`self.GetAvatarActorFromActorInfo`) null)
        (set `self.Num Points` (`KismetMathLibrary.Min` (`self.MaxNumShards`) (`self.GetAbilityLevel`))))
      (:`then_1`
        (`AbilityTask_WaitInputPress.WaitInputPress` false ; 等待技能再次进入
          (:`OnPress`
            ;[1 0.9179 0.2479] 获取鼠标位置并存储
            (bind (_asynctaskproxy _datahandle) (`TargetDataUnderMouse.CreateTargetDataUnderMouse`)
              (:`ValidData`
                (set `self.Mouse Hit Location` (`.ImpactPoint` (`GameplayStatics.BreakHitResult` (`AbilitySystemBlueprintLibrary.GetHitResultFromTargetData` _datahandle))))
                (`|ExecutionSequence`
                  (:`then_0`
                    ;[1 1 1] 出生点集合 和 获取地面点
                    (bind _returnvalue_2 (`|SpawnActorFromClass` "/Game/Blueprints/AbilitySystem/_Feibi/Abilites/Arcane/ArcaneShards/BP_PointCollection.BP_PointCollection_C" (`KismetMathLibrary.MakeTransform` (`self.Mouse Hit Location`)) "AlwaysSpawn" "MultiplyWithRoot" null null))
                    (set `self.Point Collection` _returnvalue_2)
                    (set `self.Ground Point` (`PointCollection.GetGroundPoints` (`self.Point Collection`) (`self.Mouse Hit Location`) (`self.Num Points`) (`KismetMathLibrary.RandomFloatInRange` 0.0 360.0))))
                  (:`then_1`
                    ;[0 1 0.5711] 处理蒙太奇有关
                    (message `CombatInterface.UpdateFacingTarget` (`self.GetAvatarActorFromActorInfo`) (`self.Mouse Hit Location`))
                    (`AbilityTask_PlayMontageAndWait.CreatePlayMontageAndWaitProxy` "None" "/Game/Assets/Characters/Feibi/Anim/AM_JumpAttack.AM_JumpAttack" 1.0 "None" false
                      (:`then`
                        (`AbilityTask_WaitGameplayEvent.WaitGameplayEvent` (struct :`TagName` "Event.Montage.ArcaneShards") null true
                          (:`EventReceived`
                            (bind _returnvalue_3 (`KismetSystemLibrary.K2_SetTimerDelegate` (delegate `SpawnShard`) (`self.SharSpawnDeltaTime`) true)) ; 使用定时器循环生成个体
                            (set `self.ShardSpawnTimer` _returnvalue_3)
                            (`self.SpawnShard`) ; 调用一次事件,触发后生成一个个体
                            (message `PlayerInterface.HideMagicCircle` (`self.GetAvatarActorFromActorInfo`)) ; 隐藏光圈
                            (`self.K2_CommitAbilityCost` false)))))))))))))))

(event `SpawnShard`
  (bind _returnvalue (`self.GetAvatarActorFromActorInfo`))
  (if (< (`self.Count`) (`self.Num Points`))
    (set `self.ShardSpawnLocation` (`SceneComponent.K2_GetComponentLocation` (`|GetArrayItem` (`self.Ground Point`) (`self.Count`)))) ; 设置技能位置
    (`self.K2_ExecuteGameplayCueWithParams` (struct :`TagName` "GameplayCue.ArcaneShards") (`AbilitySystemBlueprintLibrary.MakeGameplayCueParameters` 0.0 0.0 (struct) (struct) (struct) (struct) (struct) (`self.ShardSpawnLocation`))) ; 播放技能效果
    (`/Engine/EditorBlueprintResources/StandardMacros.IncrementInt` (`self.Count`)
      (:`  `
        (bind _outoverlappingactors (`AuraAbilitySystemLibrary.GetLivePlayersWithinRadius` _returnvalue (`|MakeArray` _returnvalue) (`self.RadialDamageOuterRadius`) (`self.ShardSpawnLocation`))) ; 获取技能可以命中的目标
        (bind _output_get (set `self.PlayerToDamage` _outoverlappingactors)) ; 保存变量防止多次调用前面节点
        (for _array_element _output_get
          (bind _returnvalue_2 (- (`Actor.K2_GetActorLocation` _array_element) (`self.ShardSpawnLocation`)))
          (`AuraAbilitySystemLibrary.ApplyDamageEffect` (`self.MakeDamageEffectParamsFromClassDefaults` _array_element (`self.ShardSpawnLocation`) true _returnvalue_2 true _returnvalue_2 true 35.0)) ; 应用伤害
        )))
    (else
      (`KismetSystemLibrary.K2_ClearAndInvalidateTimerHandle` (`self.ShardSpawnTimer`))
      (`Actor.K2_DestroyActor` (`self.Point Collection`))
      (`self.K2_CommitAbilityCooldown` false)
      (`self.K2_EndAbility`))))