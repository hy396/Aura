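; Electrocute gameplay ability: a held lightning beam from the caster to the target under the mouse, chaining to additional targets if it has CombatInterface.
; A montage event locks movement, adds ShockLoop cues and starts a looping timer that commits cost and damages all targets.
; Release (server-delayed by MinSpellTime), primary death or failed cost ends it, applying final damage and cooldown.
; Additional target deaths only remove that target's link.
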(event `self.K2_ActivateAbility`
  (`self.EnforcelmplementsCombatInterface`)
  ;[0.1356 0.000304 1] 存储鼠标数据变量
  (bind (_asynctaskproxy _datahandle) (`TargetDataUnderMouse.CreateTargetDataUnderMouse`)
    (:`ValidData`
      (`self.StoreMouseDataInfo` (`AbilitySystemBlueprintLibrary.GetHitResultFromTargetData` _datahandle))
      (`self.StoreOwnerVariables`)
      (`|ExecutionSequence`
        (:`then_0`
          (set `PlayerController.bShowMouseCursor` false (`self.OwnerPlayerController`))
          (message `CombatInterface.UpdateFacingTarget` (`self.GetAvatarActorFromActorInfo`) (`self.MouseHitLocation`))
          (`self.K2_ExecuteGameplayCue` (struct :`TagName` "GameplayCue.ShockBrust"))
          (`AbilityTask_PlayMontageAndWait.CreatePlayMontageAndWaitProxy` "None" (`self.Montage_Electrocute`) 1.0 "None" false
            (:`then`
              (`AbilityTask_WaitGameplayEvent.WaitGameplayEvent` (struct :`TagName` "Event.Montage.Electrocute") null true
                (:`EventReceived`
                  (`self.InShockLoop`)
                  (`self.Spawn Electric Beam`)
                  (bind _returnvalue (`KismetSystemLibrary.K2_SetTimerDelegate` (delegate `DamageAndCost`) (`self.DamageDeltaTime`) true))
                  (set `self.DamageAndCostTimer` _returnvalue))))))
        (:`then_1`
          (bind (_asynctaskproxy_2 _timeheld) (`AbilityTask_WaitInputRelease.WaitInputRelease` false)
            (:`OnRelease`
              (set `self.Time Held` _timeheld)
              (if (< (`self.Time Held`) (`self.MinSpellTime`))
                (`self.K2_HasAuthority`
                  (:`True`
                    (`KismetSystemLibrary.Delay` (`self.MinSpellTime`))
                    (`self.PrepareToEndAbility` :!label _label)
                    (`self.Clear Timer End Ability`))
                  (:`False`
                    (`self.PrepareToEndAbility`)))
                (else
                  (goto _label))))))))))

(event `DamageAndCost`
  (bind _returnvalue (message `CombatInterface.IsDead` (`self.MouseHitActor`)))
  (if _returnvalue
    (`self.PrepareToEndAbility`)
    (`self.Clear Timer End Ability`)
    (else
      (bind _returnvalue_2 (`self.K2_CommitAbilityCost` false)) ; 如果蓝量不足，也会直接结束技能
      (if _returnvalue_2
        (`self.Apply Damage`)
        (else
          (`self.PrepareToEndAbility`)
          (`self.Clear Timer End Ability`))))))

(event `self.PrimaryTargetDied`
  (params (DeadActor :type "Actor Object Reference"))
  ;[1 1 1] 主要目标死亡时，结束技能
  (`self.PrepareToEndAbility`)
  (`self.Clear Timer End Ability`))

(event `self.AdditionalTargetDied`
  (params (DeadActor :type "Actor Object Reference"))
  ;[1 1 1] 额外的目标死亡时，将额外目标清除和表现效果，技能继续执行
  (`self.RemoveAddtitionalCue` DeadActor)
  (`KismetArrayLibrary.Array_RemoveItem` (`self.Additional Targets`) DeadActor))

(fn `AddShockLoopCuetoAdditionalTarget`
  (params (`Additional Target` :type "Actor Object Reference"))
  (locals (TargetActor :type "Actor Object Reference"))
  (bind _targetactor (`local.TargetActor`))
  (bind _returnvalue (`AbilitySystemBlueprintLibrary.MakeGameplayCueParameters` 0.0 0.0 (struct) (struct) (struct) (struct) (struct) (`Actor.K2_GetActorLocation` _targetactor) (0.0 0.0 0.0) null null _targetactor null 1 1 (`Actor.RootComponent` (`self.MouseHitActor`))))
  (bind _output_get (set `local.TargetActor` `Additional Target`))
  (`BlueprintMapLibrary.Map_Add` (`self.AdditionalActorsToCueParams`) _output_get _returnvalue)
  (`GameplayCueFunctionLibrary.AddGameplayCueOnActor` (`local.TargetActor`) (struct :`TagName` "GameplayCue.ShockLoop") _returnvalue))

(fn `Apply Damage`
  (`self.ApplyDamageSingleTarget` (`self.MouseHitActor`))
  (for _array_element (`self.Additional Targets`)
    (`self.ApplyDamageSingleTarget` _array_element)))

(fn `ApplyDamageSingleTarget`
  (params (Actor :type "Actor Object Reference"))
  (locals (TargetASC :type "AbilitySystemComponent Object Reference") (`Effect Spec` :type "GameplayEffectSpecHandle Structure"))
  (bind _returnvalue (`self.GetAbilitySystemComponentFromActorInfo`))
  (bind _output_get (set `local.TargetASC` (`AbilitySystemBlueprintLibrary.GetAbilitySystemComponent` Actor)))
  (if (`KismetSystemLibrary.IsValid` _output_get)
    (bind _output_get_2 (set `local.Effect Spec` (`AbilitySystemComponent.MakeOutgoingSpec` _returnvalue (`self.DamageEffectClass`) (`KismetMathLibrary.Conv_IntToDouble` (`self.GetAbilityLevel`)) (`AbilitySystemComponent.MakeEffectContext` _returnvalue))))
    (bind _returnvalue_2 (`AbilitySystemBlueprintLibrary.AssignTagSetByCallerMagnitude` _output_get_2 (`self.DamageType`) (`self.GetDamageAtLevel`)))
    (`AbilitySystemComponent.BP_ApplyGameplayEffectSpecToSelf` (`local.TargetASC`) _returnvalue_2) ; 应用GE
  ))

(fn `Clear Timer End Ability`
  (`BlueprintMapLibrary.Map_Clear` (`self.AdditionalActorsToCueParams`))
  (`KismetArrayLibrary.Array_Clear` (`self.Additional Targets`))
  (`self.K2_CommitAbilityCooldown` false)
  (`KismetSystemLibrary.K2_ClearAndInvalidateTimerHandle` (`self.DamageAndCostTimer`))
  (`self.K2_EndAbility`))

(fn `EnforcelmplementsCombatInterface`
  (if (not (`KismetSystemLibrary.DoesImplementInterface` (`self.GetAvatarActorFromActorInfo`) "/Script/Aura.CombatInterface"))
    (`self.K2_EndAbility`)))

(fn `InShockLoop`
  (message `CombatInterface.SetInShockLoop` (`self.GetAvatarActorFromActorInfo`) true)
  (`CharacterMovementComponent.DisableMovement` (`Character.CharacterMovement` (`self.OwnerCharacter`))) ; 禁止移动
)

(fn `PrepareToEndAbility`
  (bind _mousehitactor (`self.MouseHitActor`))
  (set `PlayerController.bShowMouseCursor` true (`self.OwnerPlayerController`))
  (message `CombatInterface.SetInShockLoop` (`self.GetAvatarActorFromActorInfo`) false)
  (`CharacterMovementComponent.SetMovementMode` (`Character.CharacterMovement` (`self.OwnerCharacter`)) "MOVE_Walking" 0)
  (`self.OnEndAbility` (`self.Additional Targets`))
  (if (`self.FirstTargetImplements Interface`)
    (message `CombatInterface.SetIsBeingShocked` _mousehitactor false)
    (`GameplayCueFunctionLibrary.RemoveGameplayCueOnActor` _mousehitactor (struct :`TagName` "GameplayCue.ShockLoop") (`self.FirstTargetCueParams`)) ; 目标身上删除
    (`self.K2_HasAuthority`
      (:`True`
        (`AuraAbilitySystemLibrary.ApplyDamageEffect` (`self.MakeDamageEffectParamsFromClassDefaults` _mousehitactor)))
      (:`False`
        _))
    (for _array_element (`self.Additional Targets`)
      (`self.RemoveAddtitionalCue` _array_element)
      (message `CombatInterface.SetIsBeingShocked` _array_element false)
      (`self.K2_HasAuthority`
        (:`True`
          (`AuraAbilitySystemLibrary.ApplyDamageEffect` (`self.MakeDamageEffectParamsFromClassDefaults` _array_element)))))
    (else
      (`GameplayCueFunctionLibrary.RemoveGameplayCueOnActor` (`self.GetAvatarActorFromActorInfo`) (struct :`TagName` "GameplayCue.ShockLoop") (`self.FirstTargetCueParams`)) ; 目标非生物，自己身上删除
    )))

(fn `RemoveAddtitionalCue`
  (params (`Additional Actor` :type "Actor Object Reference"))
  (bind (_value _returnvalue) (`BlueprintMapLibrary.Map_Find` (`self.AdditionalActorsToCueParams`) `Additional Actor`))
  (if _returnvalue
    (`GameplayCueFunctionLibrary.RemoveGameplayCueOnActor` `Additional Actor` (struct :`TagName` "GameplayCue.ShockLoop") _value)))

(fn `Spawn Electric Beam`
  (locals (CueTarget :type "Actor Object Reference"))
  (`self.TraceFirstTarget` (`self.MouseHitLocation`))
  (bind _returnvalue (message `CombatInterface.GetWeapon` (`self.GetAvatarActorFromActorInfo`)))
  (set `self.FirstTargetCueParams` (`AbilitySystemBlueprintLibrary.MakeGameplayCueParameters` 0.0 0.0 (struct) (struct) (struct) (struct) (struct) (`self.MouseHitLocation`) (0.0 0.0 0.0) null null (`self.MouseHitActor`) null 1 1 _returnvalue))
  ;[1 1 1] 击中目标是否是拥有战斗接口
  (bind _output_get (set `self.FirstTargetImplements Interface` (`KismetSystemLibrary.DoesImplementInterface` (`self.MouseHitActor`) "/Script/Aura.CombatInterface")))
  (if _output_get
    (set `local.CueTarget` (`self.MouseHitActor`))
    (else
      (set `local.CueTarget` (`self.GetAvatarActorFromActorInfo`))))
  (`GameplayCueFunctionLibrary.AddGameplayCueOnActor` (`local.CueTarget`) (struct :`TagName` "GameplayCue.ShockLoop") (`self.FirstTargetCueParams`))
  (if (`self.FirstTargetImplements Interface`)
    (message `CombatInterface.SetIsBeingShocked` (`local.CueTarget`) true)
    (bind _outadditionaltargets (`self.StoreAdditionalTargets`))
    (bind _output_get_2 (set `self.Additional Targets` _outadditionaltargets))
    (for _array_element _output_get_2
      (message `CombatInterface.SetIsBeingShocked` _array_element true)
      (`self.AddShockLoopCuetoAdditionalTarget` _array_element))))