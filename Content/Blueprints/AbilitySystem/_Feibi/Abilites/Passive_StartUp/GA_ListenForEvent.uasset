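; Passive GameplayAbility that listens for gameplay events under the Attributes tag and turns them into attribute changes on its owner.
; On activation it waits for events matching Attributes or its child tags.
; Each event builds an EventBasedEffectClass spec with all EventTags SetByCaller magnitudes zeroed.
; It then sets the received tag's magnitude to the event's value and applies the spec to itself.
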(event `self.K2_ActivateAbility`
  (`KismetSystemLibrary.PrintString` "Listen for Event Activated")
  (bind (_asynctaskproxy _payload) (`AbilityTask_WaitGameplayEvent.WaitGameplayEvent` (struct :`TagName` "Attributes") null false false)
    (:`EventReceived`
      (bind _ge_spec (`self.Make GE Spec`))
      (bind (_eventtag _instigator _target _optionalobject _optionalobject2 _contexthandle _instigatortags _targettags _eventmagnitude) (break `GameplayEventData` _payload))
      (bind _returnvalue (`AbilitySystemBlueprintLibrary.AssignTagSetByCallerMagnitude` _ge_spec _eventtag _eventmagnitude))
      (`AbilitySystemComponent.BP_ApplyGameplayEffectSpecToSelf` (`self.GetAbilitySystemComponentFromActorInfo`) _returnvalue))))

(fn `Make GE Spec`
  (returns (`GE Spec` :type "GameplayEffectSpecHandle Structure"))
  (bind _returnvalue (`self.GetAbilitySystemComponentFromActorInfo`))
  (set `self.GE Spec` (`AbilitySystemComponent.MakeOutgoingSpec` _returnvalue (`self.EventBasedEffectClass`) 1.0 (`AbilitySystemComponent.MakeEffectContext` _returnvalue)))
  (for _array_element (`self.Event Tags`)
    (`AbilitySystemBlueprintLibrary.AssignTagSetByCallerMagnitude` (`self.GE Spec`) _array_element))
  (return (`self.GE Spec`)))