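; BP_MapEntrance_Child is a map entrance Blueprint variant that lights up when highlighted.
; HighlightActor shows its two point lights and UnHighlightActor hides them, without propagating visibility to child components.
; BeginPlay and Tick are disabled stubs, and the construction script only calls the parent's.
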(event `HighlightInterface.HighlightActor`
  (`SceneComponent.SetVisibility` (`self.PointLight1`) true false)
  (`SceneComponent.SetVisibility` (`self.PointLight`) true false))

(event `HighlightInterface.UnHighlightActor`
  (`SceneComponent.SetVisibility` (`self.PointLight`) false false)
  (`SceneComponent.SetVisibility` (`self.PointLight1`) false false))

(fn `UserConstructionScript`
  (`parent.UserConstructionScript`))