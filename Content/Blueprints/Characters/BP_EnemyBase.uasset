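; Base enemy character Blueprint that handles spawn, dissolve and death visuals, attack-facing motion warping and loot drops.
; Timelines drive a volume-preserving squash-and-stretch spawn scale and dissolve material parameters, while destruction bursts Niagara effects at the head and weapon.
; SpawnLoot gets items from loot tiers, then a looping timer spawns them one by one at evenly fanned, random distances around the enemy.
; Flagged loot takes the player's level.
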(event `self.ReceiveBeginPlay`
  (bind (_direction _scaletrack) (`Timeline|SpawnTimeline` :!via `PlayFromStart`)
    (:`Update`
      (bind _returnvalue (/ 1.0 _scaletrack))
      (`SceneComponent.SetRelativeScale3D` (`self.Mesh`) (`KismetMathLibrary.MakeVector` _returnvalue _returnvalue _scaletrack)))))

(event `self.StartDissolveTimeline`
  (params (DynamicMaterialInstance :type "Array of MaterialInstanceDynamic Object Reference (by ref)"))
  (bind (_direction _dissolvetrack) (`Timeline|DissolveTimeline` :!via `PlayFromStart`)
    (:`Update`
      (for _array_element DynamicMaterialInstance
        (`MaterialInstanceDynamic.SetScalarParameterValue` _array_element "Dissolve" _dissolvetrack)))))

(event `self.ReceiveDestroyed`
  (bind _weapon (`self.Weapon`))
  ;[1 1 1] 死亡爆头，爆武器
  (`NiagaraFunctionLibrary.SpawnSystemAtLocation` "/Game/Assets/_Niagara/Effect/NiagaraSystems/DarkBullet/NS_DarkHit_01.NS_DarkHit_01" (`SceneComponent.GetSocketLocation` (`self.Mesh`) "Head") (struct) (0.75 0.75 0.75))
  (`/Engine/EditorBlueprintResources/StandardMacros.IsValid` _weapon
    (:`Is Valid`
      (`NiagaraFunctionLibrary.SpawnSystemAtLocation` "/Game/Assets/_Niagara/Effect/NiagaraSystems/DarkBullet/NS_DarkHit_01.NS_DarkHit_01" (`SceneComponent.K2_GetComponentLocation` _weapon) (struct) (0.25 0.25 0.25)))))

(event `CombatInterface.UpdateFacingTarget`
  (params (Target :type "Vector Structure (by ref)"))
  (`MotionWarpingComponent.AddOrUpdateWarpTargetFromLocation` (`self.MotionWarping`) "FacingTarget" Target))

(event `self.SpawnLoot`
  (bind _returnvalue (`AuraAbilitySystemLibrary.GetLootTiers` null))
  (`/Engine/EditorBlueprintResources/StandardMacros.IsValid` _returnvalue
    (:`Is Valid`
      (bind _returnvalue_2 (`LootTiers.GetLootItems` _returnvalue))
      (bind _output_get (set `self.Loot Item` _returnvalue_2))
      (set `self.Loot Rotations` (`self.Get Loot Rotations` _output_get))
      (set `self.Spawn Loot Count` 0)
      (bind _returnvalue_3 (`KismetSystemLibrary.K2_SetTimerDelegate` (delegate `SpawnLootItem`) 0.1 true))
      (set `self.Loot Timer` _returnvalue_3)
      (`self.SpawnLootItem`))))

(event `SpawnLootItem`
  (bind (_lootclass _blootleveloverride) (break `LootItem` (`|GetArrayItem` (`self.Loot Item`) (`self.Spawn Loot Count`))))
  (bind _returnvalue (`|SpawnActorFromClass` _lootclass (`self.Get Loot Transform` (`self.Spawn Loot Count`)) "AdjustIfPossibleButAlwaysSpawn" "MultiplyWithRoot" null null))
  (`/Engine/EditorBlueprintResources/StandardMacros.IsValid` _returnvalue
    (:`Is Valid`
      (`self.Update Loot Level` _returnvalue _blootleveloverride))
    (:`Is Not Valid`
      _))
  (bind _result (`/Engine/EditorBlueprintResources/StandardMacros.IncrementInt` (`self.Spawn Loot Count`))
    (:`  `
      (if (>= _result (`KismetArrayLibrary.Array_Length` (`self.Loot Item`)))
        (`KismetSystemLibrary.K2_ClearAndInvalidateTimerHandle` (`self.Loot Timer`))))))

(fn `Get Loot Rotations`
  (params (TargetArray :type "Array of LootItem Structure (by ref)"))
  (returns (ReturnValue :type "Array of Rotator Structure"))
  (return (`AuraAbilitySystemLibrary.EvenlySpacedRotators` (`self.GetActorForwardVector`) (`KismetMathLibrary.Vector_Up`) 360.0 (`KismetArrayLibrary.Array_Length` TargetArray))))

(fn `Get Loot Transform`
  (params (`In Count` :type Integer))
  (returns (`Return Value` :type "Transform Structure"))
  (bind _output (`|GetArrayItem` (`self.Loot Rotations`) `In Count`))
  (bind (_returnvalue_x _returnvalue_y) (`KismetMathLibrary.BreakVector` (+ (* (`KismetMathLibrary.GetForwardVector` _output) (`KismetMathLibrary.RandomFloatInRange` (`self.MinSpawnDistance`) (`self.MaxSpawnDistance`))) (`self.K2_GetActorLocation`))))
  (return (`KismetMathLibrary.MakeTransform` (`KismetMathLibrary.MakeVector` _returnvalue_x _returnvalue_y 50.0) _output)))

(fn `Update Loot Level`
  (params (Object :type "Actor Object Reference") (Condition :type Boolean))
  (if Condition
    (bind _asaura_effect_actor (cast `AuraEffectActor` Object))
    (`/Engine/EditorBlueprintResources/StandardMacros.IsValid` _asaura_effect_actor
      (:`Is Valid`
        (bind _returnvalue (`CombatInterface.GetPlayerLevel`))
        (set `AuraEffectActor.ActorLevel` (`KismetMathLibrary.Conv_IntToDouble` _returnvalue) _asaura_effect_actor)))))

(fn `UserConstructionScript`)