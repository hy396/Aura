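; BP_Feibi is a playable character Blueprint that layers UI, motion warping, camera fading and shield effects onto its parent class.
; Death and checkpoint-save overrides show countdown and save-message widgets, while other events set the skill-loop flag and the FacingTarget warp location.
; Box overlaps fade camera-blocking actors out and back in through BI_FadeInterface.
; DunSphere spawns a Niagara effect where non-friendly AuraProjectiles touch the shield, without altering the projectile itself.
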(event `CombatInterface.Die`
  (params (DeathImpulse :type "Vector Structure (by ref)"))
  ;[1 1 1] 死亡倒数计时
  (`parent.Die` DeathImpulse)
  (bind _returnvalue (`|CreateWidget` "/Game/Blueprints/UI/Overlay/Subwidget/WBP_DieMessage.WBP_DieMessage_C" (`GameplayStatics.GetPlayerController` 0)))
  (`/Game/Blueprints/UI/Overlay/Subwidget/WBP_DieMessage.Set Num` _returnvalue (`KismetMathLibrary.FTrunc` (`self.DeathTime`)))
  (`UserWidget.AddToViewport` _returnvalue 0))

(event `CombatInterface.SetInShockLoop`
  (params (bInLoop :type Boolean))
  ;[1 1 1] 设置技能循环释放状态
  (set `self.InShockLoop` bInLoop))

(event `CombatInterface.UpdateFacingTarget`
  (params (Target :type "Vector Structure (by ref)"))
  ;[1 1 1] 设置朝向接口事件
  (`MotionWarpingComponent.AddOrUpdateWarpTargetFromLocation` (`self.MotionWarping`) "FacingTarget" Target))

(event `PlayerInterface.SaveProgress`
  (params (CheckpointTag :type "Name (by ref)"))
  ;[1 1 1] 存档消息弹窗
  (`parent.SaveProgress` CheckpointTag)
  (bind _savemessage (`self.SaveMessage`)
    (:`then`
      (`Widget.RemoveFromParent` _savemessage))
    (:`else`
      _))
  (bind _returnvalue (`|CreateWidget` "/Game/Blueprints/UI/Overlay/Subwidget/WBP_SaveMessage.WBP_SaveMessage_C" (`GameplayStatics.GetPlayerController` 0)))
  (bind _output_get (set `self.SaveMessage` _returnvalue))
  (`UserWidget.AddToViewport` _output_get 0))

(event `self.Box.OnComponentBeginOverlap`
  (params (OverlappedComponent :type "PrimitiveComponent Object Reference") (OtherActor :type "Actor Object Reference") (OtherComp :type "PrimitiveComponent Object Reference") (OtherBodyIndex :type Integer) (bFromSweep :type Boolean) (SweepResult :type "HitResult Structure (by ref)"))
  ;[1 1 1] 阻挡相机的actor的隐藏与打开
  (if (`KismetSystemLibrary.DoesImplementInterface` OtherActor "/Game/Blueprints/Actor/FadeActor/BI_FadeInterface.BI_FadeInterface_C")
    (message `/Game/Blueprints/Actor/FadeActor/BI_FadeInterface.FadeOut` OtherActor)))

(event `self.DunSphere.OnComponentBeginOverlap`
  (params (OverlappedComponent :type "PrimitiveComponent Object Reference") (OtherActor :type "Actor Object Reference") (OtherComp :type "PrimitiveComponent Object Reference") (OtherBodyIndex :type Integer) (bFromSweep :type Boolean) (SweepResult :type "HitResult Structure (by ref)"))
  (bind _returnvalue (`self.GetTransform` OtherActor))
  ;[1 1 1] 护盾
  (bind _asaura_projectile (cast `AuraProjectile` OtherActor))
  (bind (_worldcontextobject _damagegameplayeffectclass _sourceabilitysystemcomponent) (break `DamageEffectParams` (`AuraProjectile.DamageEffectParams` _asaura_projectile)))
  (`/Engine/EditorBlueprintResources/StandardMacros.IsValid` _sourceabilitysystemcomponent
    (:`Is Valid`
      (bind _returnvalue_2 (`ActorComponent.GetOwner` _sourceabilitysystemcomponent))
      (`/Engine/EditorBlueprintResources/StandardMacros.IsValid` _returnvalue_2
        (:`Is Valid`
          (if (`AuraAbilitySystemLibrary.IsNotFriend` _returnvalue_2 self)
            (`NiagaraFunctionLibrary.SpawnSystemAtLocation` "/Game/Assets/_Niagara/VFX/Vefects/Anime_Stylized_VFX/Skills/MagicAttacks/Fire/NS_FireMagic_Cast1.NS_FireMagic_Cast1" (`KismetMathLibrary.TransformLocation` _returnvalue) (`KismetMathLibrary.TransformRotation` _returnvalue) (0.25 0.25 0.25))))))))

(event `self.Box.OnComponentEndOverlap`
  (params (OverlappedComponent :type "PrimitiveComponent Object Reference") (OtherActor :type "Actor Object Reference") (OtherComp :type "PrimitiveComponent Object Reference") (OtherBodyIndex :type Integer))
  ;[1 1 1] 阻挡相机的actor的隐藏与打开
  (if (`KismetSystemLibrary.DoesImplementInterface` OtherActor "/Game/Blueprints/Actor/FadeActor/BI_FadeInterface.BI_FadeInterface_C")
    (message `/Game/Blueprints/Actor/FadeActor/BI_FadeInterface.FadeIn` OtherActor)))

(fn `UserConstructionScript`)